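; Prototype trigger actor that opens a sliding double door while the player's BP_ThirdPersonCharacter is in its trigger areas.
; Actor or OutDoor begin-overlap plays one Timeline, and Box or OutDoor end-overlap reverses it, with debug prints.
; The Timeline slides RightDoor and LeftDoor along relative Y and moves the trigger base and switch meshes along Z.
; Leftover disconnected gate-movement nodes never run, and the LocalSpeed flipped on finish drives no live movement.
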(event `self.ReceiveBeginPlay`
  (`KismetSystemLibrary.PrintString` "시작했을지도"))

(event `self.ReceiveActorBeginOverlap`
  (params (OtherActor :type "Actor Object Reference"))
  (bind _rightdoor (`self.RightDoor`))
  (bind _leftdoor (`self.LeftDoor`))
  (bind _sm_triggerbase (`self.SM_TriggerBase`))
  (bind _sm_switch (`self.SM_Switch`))
  (bind (_relativelocation_x _relativelocation_y _relativelocation_z) (`KismetMathLibrary.BreakVector` (`SceneComponent.RelativeLocation` _rightdoor)))
  (bind (_relativelocation_x_2 _relativelocation_y_2 _relativelocation_z_2) (`KismetMathLibrary.BreakVector` (`SceneComponent.RelativeLocation` _leftdoor)))
  (bind (_relativelocation_x_3 _relativelocation_y_3) (`KismetMathLibrary.BreakVector` (`SceneComponent.RelativeLocation` _sm_triggerbase)))
  (bind (_relativelocation_x_4 _relativelocation_y_4) (`KismetMathLibrary.BreakVector` (`SceneComponent.RelativeLocation` _sm_switch)))
  ;[1 1 1] 플레이어가 트리거 영역에 들어오면
  (bind _asbp_third_person_character (cast `/Game/ThirdPerson/Blueprints/BP_ThirdPersonCharacter` OtherActor :!label _label))
  (`/Engine/EditorBlueprintResources/StandardMacros.IsValid` _asbp_third_person_character
    (:`Is Valid`
      (if (== _asbp_third_person_character (`GameplayStatics.GetPlayerPawn` 0))
        (`KismetSystemLibrary.PrintString` "door open")
        ;[1 1 1] 문을 위에서 아래로 슬라이딩해라
        (bind (_direction _opendoorr _opendoorl _but _speed) (`Timeline|Timeline` :!label _label_2)
          (:`Update`
            (`SceneComponent.K2_SetRelativeLocation` _rightdoor (`KismetMathLibrary.MakeVector` _relativelocation_x _opendoorr _relativelocation_z) false false)
            (`SceneComponent.K2_SetRelativeLocation` _leftdoor (`KismetMathLibrary.MakeVector` _relativelocation_x_2 _opendoorl _relativelocation_z_2) false false)
            (`SceneComponent.K2_SetRelativeLocation` _sm_triggerbase (`KismetMathLibrary.MakeVector` _relativelocation_x_3 _relativelocation_y_3 _but) false false)
            (`SceneComponent.K2_SetRelativeLocation` _sm_switch (`KismetMathLibrary.MakeVector` _relativelocation_x_4 _relativelocation_y_4 _but) false false))
          (:`Finished`
            (set `self.LocalSpeed` (* (`self.LocalSpeed`) -1.0))))))))

(event `self.OutDoor.OnComponentBeginOverlap`
  (params (OverlappedComponent :type "PrimitiveComponent Object Reference") (OtherActor :type "Actor Object Reference") (OtherComp :type "PrimitiveComponent Object Reference") (OtherBodyIndex :type Integer) (bFromSweep :type Boolean) (SweepResult :type "HitResult Structure (by ref)"))
  (goto _label))

(event `self.Box.OnComponentEndOverlap`
  (params (OverlappedComponent :type "PrimitiveComponent Object Reference") (OtherActor :type "Actor Object Reference") (OtherComp :type "PrimitiveComponent Object Reference") (OtherBodyIndex :type Integer))
  (bind _asbp_third_person_character (cast `/Game/ThirdPerson/Blueprints/BP_ThirdPersonCharacter` OtherActor :!label _label_3))
  (`/Engine/EditorBlueprintResources/StandardMacros.IsValid` _asbp_third_person_character
    (:`Is Valid`
      (if (== _asbp_third_person_character (`GameplayStatics.GetPlayerPawn` 0))
        (`KismetSystemLibrary.PrintString` "door close")
        (goto _label_2 :!via `Reverse`)))))

(event `self.OutDoor.OnComponentEndOverlap`
  (params (OverlappedComponent :type "PrimitiveComponent Object Reference") (OtherActor :type "Actor Object Reference") (OtherComp :type "PrimitiveComponent Object Reference") (OtherBodyIndex :type Integer))
  (goto _label_3))

(event `self.ReceiveTick`
  (params (DeltaSeconds :type "Float (single-precision)")))

(fn `UserConstructionScript`)