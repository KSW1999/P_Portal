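; BP_Projectile3 is a prototype pellet projectile that moves itself along its forward vector.
; Each Tick applies a swept offset scaled by Dir, and a Sphere hit sets Dir to -1 to send it backward.
; Tick also re-applies a five-second lifespan every frame, continually restarting that timer.
; A custom event for a target transform is empty, with its teleport and velocity-preserving ProjectileMovement logic left disconnected.
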(event `self.ReceiveTick`
  (params (DeltaSeconds :type "Float (single-precision)"))
  (`self.SetLifeSpan` 5.0)
  (`self.K2_AddActorWorldOffset` (* (`self.GetActorForwardVector`) (`self.dir`)) true))

(event `self.Sphere.OnComponentHit`
  (params (HitComponent :type "PrimitiveComponent Object Reference") (OtherActor :type "Actor Object Reference") (OtherComp :type "PrimitiveComponent Object Reference") (NormalImpulse :type "Vector Structure") (Hit :type "HitResult Structure (by ref)"))
  (set `self.dir` -1.0))

(event `CustomEvent`
  (params (TargetLocation :type "Vector Structure") (TargetRotation :type "Rotator Structure")))

(fn `UserConstructionScript`)