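; BP_Projectile1 is a prototype pellet projectile that expires seven seconds after spawning and can jump through portals.
; Its JumpPortal event moves it to a target location, passing no rotation, and resets the projectile movement velocity along the actor's forward vector.
; The pre-jump speed is stored to preserve velocity, but the multiply that would apply it is unused, so only the unit forward vector is assigned.
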(event `self.ReceiveBeginPlay`
  ;[1 1 1] Pellet lifetime = 7sec
  (`self.SetLifeSpan` 7.0))

(event `/Game/BP/Portal/BPI_PortalJumper.JumpPortal`
  (params (TargetLocation :type "Vector Structure") (TargetRotation :type "Rotator Structure"))
  ;[1 1 1] Keep the velocity when Pellet go through the Portal
  (set `self.JumpVelocity` (`KismetMathLibrary.VSize` (`SceneComponent.GetComponentVelocity` (`self.CollisionComponent`))))
  (`self.K2_SetActorLocationAndRotation` TargetLocation)
  (set `MovementComponent.Velocity` (`self.GetActorForwardVector`) (`self.ProjectileMovement1`)))

(fn `UserConstructionScript`)