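; BP_Projectile2 is a prototype pellet projectile that can travel through portals.
; Tick restarts a five-second lifespan and nudges it forward each frame without sweep, while Hit applies one mirrored-vector offset without changing its rotation.
; JumpPortal teleports it to a target transform and redirects ProjectileMovement velocity along the new forward, preserving speed.
; A PelletLifetime timeline for moving the collision component is disconnected.
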(event `self.ReceiveTick`
  (params (DeltaSeconds :type "Float (single-precision)"))
  (`self.SetLifeSpan` 5.0)
  (`self.K2_AddActorWorldOffset` (`self.GetActorForwardVector`)))

(event `self.ReceiveHit`
  (params (MyComp :type "PrimitiveComponent Object Reference") (Other :type "Actor Object Reference") (OtherComp :type "PrimitiveComponent Object Reference") (bSelfMoved :type Boolean) (HitLocation :type "Vector Structure") (HitNormal :type "Vector Structure") (NormalImpulse :type "Vector Structure") (Hit :type "HitResult Structure (by ref)"))
  (`self.K2_AddActorWorldOffset` (`KismetMathLibrary.MirrorVectorByNormal` (`self.GetActorForwardVector`) HitNormal)))

(event `/Game/BP/Portal/BPI_PortalJumper.JumpPortal`
  (params (TargetLocation :type "Vector Structure") (TargetRotation :type "Rotator Structure"))
  (set `self.JumpVelocity` (`KismetMathLibrary.VSize` (`SceneComponent.GetComponentVelocity` (`MovementComponent.UpdatedPrimitive` (`self.ProjectileMovement`)))))
  (`self.K2_SetActorLocationAndRotation` TargetLocation TargetRotation)
  (set `MovementComponent.Velocity` (* (`self.GetActorForwardVector`) (`self.JumpVelocity`)) (`self.ProjectileMovement`)))

(fn `UserConstructionScript`)