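; BP_Lift is a prototype lift that lowers on external activation and rises when something overlaps its trigger box.
; LiftActivated increments a pressure counter; reaching the threshold plays a timeline driving the Cube's relative Z, while lower counts reverse it.
; Box overlap plays a door sound and a second Z timeline, which reverses after a short delay, without checking the overlapping actor or whether the lift is down.
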(event `Lift Activated`
  (bind _cube (`self.Cube`))
  (bind (_relativelocation_x _relativelocation_y) (`KismetMathLibrary.BreakVector` (`SceneComponent.RelativeLocation` _cube)))
  ;[1 1 1] Lift Down when LiftOpen Collision Activated
  (`/Engine/EditorBlueprintResources/StandardMacros.IncrementInt` (`self.Pressure to activate Lift`)
    (:`  `
      (if (>= (`self.Pressure to activate Lift`) (`self.Pressure needed to activate Lift`))
        (if (`self.isLiftDown`)
          (bind (_direction _gate_activation) (`Timeline|Pellet Receive Lift Down` :!label _label)
            (:`Update`
              (`SceneComponent.K2_SetRelativeLocation` _cube (`KismetMathLibrary.MakeVector` _relativelocation_x _relativelocation_y _gate_activation) false false))
            (:`Finished`
              (set `self.isLiftDown` true)))
          (else
            (`GameplayStatics.PlaySound2D` "/Game/BP/Sounds/Doors/doormove2.doormove2" 1.0 1.0 0.0 null null)
            (goto _label)))
        (else
          (goto _label :!via `Reverse`))))))

(event `self.Box.OnComponentEndOverlap`
  (params (OverlappedComponent :type "PrimitiveComponent Object Reference") (OtherActor :type "Actor Object Reference") (OtherComp :type "PrimitiveComponent Object Reference") (OtherBodyIndex :type Integer)))

(event `self.Box.OnComponentBeginOverlap`
  (params (OverlappedComponent :type "PrimitiveComponent Object Reference") (OtherActor :type "Actor Object Reference") (OtherComp :type "PrimitiveComponent Object Reference") (OtherBodyIndex :type Integer) (bFromSweep :type Boolean) (SweepResult :type "HitResult Structure (by ref)"))
  (bind _cube (`self.Cube`))
  (bind (_relativelocation_x _relativelocation_y) (`KismetMathLibrary.BreakVector` (`SceneComponent.RelativeLocation` _cube)))
  ;[1 1 1] Lift Up when Player is on the lift
  (`GameplayStatics.PlaySound2D` "/Game/BP/Sounds/Doors/doormove2.doormove2" 1.0 1.0 0.0 null null)
  (bind (_direction _newtrack_3) (`Timeline|Lift Up down` :!label _label_2)
    (:`Update`
      (`SceneComponent.K2_SetRelativeLocation` _cube (`KismetMathLibrary.MakeVector` _relativelocation_x _relativelocation_y _newtrack_3) false false))
    (:`Finished`
      (`KismetSystemLibrary.Delay` 2.5)
      (goto _label_2 :!via `Reverse`))))

(fn `UserConstructionScript`)