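; BP_GateOpen is a pressure switch that signals a referenced gate when an actor overlaps it or leaves it.
; Begin and end overlap call the gate's activate and deactivate functions, each playing a 2D button sound, with no filtering of the overlapping actor.
; The SwitchActivate timeline plays forward or in reverse to drive the button mesh's relative Z, pressing it down and popping it back up.
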(event `self.ReceiveActorBeginOverlap`
  (params (OtherActor :type "Actor Object Reference"))
  (bind _button (`self.Button`))
  (bind (_relativelocation_x _relativelocation_y) (`KismetMathLibrary.BreakVector` (`SceneComponent.RelativeLocation` _button)))
  ;[1 1 1] When Overlapped, switch activated
  (`/Game/Proto/Stage/BP_Gate.SwtichActivated` (`self.Gate to Activate`))
  (`GameplayStatics.PlaySound2D` "/Game/BP/Sounds/Buttons/pressure_button_down_01.pressure_button_down_01" 0.5 1.0 0.0 null null)
  (bind (_direction _switch_position) (`Timeline|Switch Activate` :!label _label)
    (:`Update`
      ;[1 1 1] Button pressed down and pops up
      (`SceneComponent.K2_SetRelativeLocation` _button (`KismetMathLibrary.MakeVector` _relativelocation_x _relativelocation_y _switch_position) false false))))

(event `self.ReceiveActorEndOverlap`
  (params (OtherActor :type "Actor Object Reference"))
  ;[1 1 1] When Overlap ends, switch deactivated
  (`/Game/Proto/Stage/BP_Gate.SwitchDeactivated` (`self.Gate to Activate`))
  (`GameplayStatics.PlaySound2D` "/Game/BP/Sounds/Buttons/pressure_button_up_01.pressure_button_up_01" 0.5 1.0 0.0 null null)
  (goto _label :!via `Reverse`))

(fn `UserConstructionScript`)