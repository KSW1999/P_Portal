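; BP_Dropper is a stage actor with a two-part gate that slides open and closed on external open and close events.
; The GateActivation timeline plays to open and reverses to close, driving the relative X of GateRight and GateRightL in opposite directions.
; Pressure button counting against a required total is present but disconnected, so it never affects the gate.
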(event `Door Open Activation`
  (bind _gate_right (`self.Gate_Right`))
  (bind _gate_right_l (`self.Gate_Right_L`))
  (bind (_relativelocation_x _relativelocation_y _relativelocation_z) (`KismetMathLibrary.BreakVector` (`SceneComponent.RelativeLocation` _gate_right_l)))
  (bind (_relativelocation_x_2 _relativelocation_y_2 _relativelocation_z_2) (`KismetMathLibrary.BreakVector` (`SceneComponent.RelativeLocation` _gate_right)))
  (bind (_direction _gate_activation) (`Timeline|Gate Activation` :!label _label)
    (:`Update`
      (`SceneComponent.K2_SetRelativeLocation` _gate_right (`KismetMathLibrary.MakeVector` _gate_activation _relativelocation_y_2 _relativelocation_z_2) false false)
      (`SceneComponent.K2_SetRelativeLocation` _gate_right_l (`KismetMathLibrary.MakeVector` (* _gate_activation -1.0) _relativelocation_y _relativelocation_z) false false))))

(event `Door Close Activation`
  (goto _label :!via `Reverse`))

(fn `UserConstructionScript`)