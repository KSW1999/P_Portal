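; BP_Gate is a two-panel stage gate that opens once enough pressure switches are active.
; Switch activated and deactivated events raise or lower an active count, then compare it to the required number.
; At or above that number the GateActivation timeline plays, otherwise it reverses.
; Its track slides the right and left panels apart along relative X, mirrored by negation.
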(event `SwtichActivated`
  (bind _gate_right (`self.Gate_Right`))
  (bind _gate_right_l (`self.Gate_Right_L`))
  (bind (_relativelocation_x _relativelocation_y _relativelocation_z) (`KismetMathLibrary.BreakVector` (`SceneComponent.RelativeLocation` _gate_right_l)))
  (bind (_relativelocation_x_2 _relativelocation_y_2 _relativelocation_z_2) (`KismetMathLibrary.BreakVector` (`SceneComponent.RelativeLocation` _gate_right)))
  ;[1 1 1] Gate opens when PressureButtonActivate is equal or greater than PressureButtonNeeded
  (`/Engine/EditorBlueprintResources/StandardMacros.IncrementInt` (`self.PressureButtonActivate`)
    (:`  `
      (if (>= (`self.PressureButtonActivate`) (`self.PressureButtonNeeded`))
        (bind (_direction _gate_activation) (`Timeline|Gate Activation` :!label _label)
          (:`Update`
            ;[1 1 1] Right Gate New Location
            (`SceneComponent.K2_SetRelativeLocation` _gate_right (`KismetMathLibrary.MakeVector` _gate_activation _relativelocation_y_2 _relativelocation_z_2) false false)
            ;[1 1 1] Left Gate New Location
            (`SceneComponent.K2_SetRelativeLocation` _gate_right_l (`KismetMathLibrary.MakeVector` (* _gate_activation -1.0) _relativelocation_y _relativelocation_z) false false)))
        (else
          (goto _label :!via `Reverse`))))))

(event `SwitchDeactivated`
  ;[1 1 1] Gate closes when PressureButtonActivate is equal or greater than PressureButtonNeeded
  (`/Engine/EditorBlueprintResources/StandardMacros.DecrementInt` (`self.PressureButtonActivate`)
    (:`  `
      (if (>= (`self.PressureButtonActivate`) (`self.PressureButtonNeeded`))
        (goto _label)
        (else
          (goto _label :!via `Reverse`))))))

(fn `UserConstructionScript`)