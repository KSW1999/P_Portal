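; BP_AutoGate is a portal gate whose two doors slide shut when something overlaps its trigger box.
; The overlap plays a door sound and runs the CloseDoor timeline, which drives the relative X of the left and right door components.
; IsDoorClose is set only when the timeline finishes, blocking further triggers after that; the gate has no reopening logic.
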(event `self.ReceiveBeginPlay`
  (set `self.isDoorClose` false))

(event `self.Box.OnComponentBeginOverlap`
  (params (OverlappedComponent :type "PrimitiveComponent Object Reference") (OtherActor :type "Actor Object Reference") (OtherComp :type "PrimitiveComponent Object Reference") (OtherBodyIndex :type Integer) (bFromSweep :type Boolean) (SweepResult :type "HitResult Structure (by ref)"))
  (bind _finalportaldoor_door_right (`self.FinalPortalDoor_Door_Right`))
  (bind _finalportaldoor_door_left (`self.FinalPortalDoor_Door_Left`))
  (bind (_relativelocation_x _relativelocation_y _relativelocation_z) (`KismetMathLibrary.BreakVector` (`SceneComponent.RelativeLocation` _finalportaldoor_door_right)))
  (bind (_relativelocation_x_2 _relativelocation_y_2 _relativelocation_z_2) (`KismetMathLibrary.BreakVector` (`SceneComponent.RelativeLocation` _finalportaldoor_door_left)))
  ;[1 1 1] 박스에 닿으면 양쪽 문이 닫힌다
  (if (not (`self.isDoorClose`))
    (`GameplayStatics.PlaySound2D` "/Game/BP/Sounds/Doors/doormove2.doormove2" 0.5 1.0 0.0 null null)
    (bind (_direction _right _left) (`Timeline|CloseDoor`)
      (:`Update`
        (`SceneComponent.K2_SetRelativeLocation` _finalportaldoor_door_right (`KismetMathLibrary.MakeVector` _right _relativelocation_y _relativelocation_z) false false)
        (`SceneComponent.K2_SetRelativeLocation` _finalportaldoor_door_left (`KismetMathLibrary.MakeVector` _left _relativelocation_y_2 _relativelocation_z_2) false false))
      (:`Finished`
        (set `self.isDoorClose` true)))))

(fn `UserConstructionScript`)