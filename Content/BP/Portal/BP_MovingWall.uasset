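; BP_MovingWall is a portal-area moving wall that shifts PortalPlace pieces vertically in two trigger-driven stages.
; Overlapping Box plays a timeline whose Move track sets the relative Z of all four PortalPlace components.
; Overlapping Box1 plays a second timeline that moves PortalPlace2 through 4 again, plus PushingCyl4 through 6 on a separate Move2 track.
; Neither overlap checks the entering actor or reverses its timeline.
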(event `self.Box1.OnComponentBeginOverlap`
  (params (OverlappedComponent :type "PrimitiveComponent Object Reference") (OtherActor :type "Actor Object Reference") (OtherComp :type "PrimitiveComponent Object Reference") (OtherBodyIndex :type Integer) (bFromSweep :type Boolean) (SweepResult :type "HitResult Structure (by ref)"))
  (bind _pushingcyl4 (`self.PushingCyl4`))
  (bind _pushingcyl5 (`self.PushingCyl5`))
  (bind _pushingcyl6 (`self.PushingCyl6`))
  (bind _portalplace2 (`self.PortalPlace2`))
  (bind _portalplace3 (`self.PortalPlace3`))
  (bind _portalplace4 (`self.PortalPlace4`))
  (bind (_relativelocation_x _relativelocation_y) (`KismetMathLibrary.BreakVector` (`SceneComponent.RelativeLocation` _pushingcyl6)))
  (bind (_relativelocation_x_2 _relativelocation_y_2) (`KismetMathLibrary.BreakVector` (`SceneComponent.RelativeLocation` _portalplace4)))
  (bind (_relativelocation_x_3 _relativelocation_y_3) (`KismetMathLibrary.BreakVector` (`SceneComponent.RelativeLocation` _pushingcyl4)))
  (bind (_relativelocation_x_4 _relativelocation_y_4) (`KismetMathLibrary.BreakVector` (`SceneComponent.RelativeLocation` _pushingcyl5)))
  (bind (_relativelocation_x_5 _relativelocation_y_5) (`KismetMathLibrary.BreakVector` (`SceneComponent.RelativeLocation` _portalplace2)))
  (bind (_relativelocation_x_6 _relativelocation_y_6) (`KismetMathLibrary.BreakVector` (`SceneComponent.RelativeLocation` _portalplace3)))
  (bind (_direction _move _move2) (`Timeline|Timeline_0`)
    (:`Update`
      ;[1 1 1] 2차 트리거
      (`SceneComponent.K2_SetRelativeLocation` _portalplace2 (`KismetMathLibrary.MakeVector` _relativelocation_x_5 _relativelocation_y_5 _move) false false)
      (`SceneComponent.K2_SetRelativeLocation` _portalplace3 (`KismetMathLibrary.MakeVector` _relativelocation_x_6 _relativelocation_y_6 _move) false false)
      (`SceneComponent.K2_SetRelativeLocation` _portalplace4 (`KismetMathLibrary.MakeVector` _relativelocation_x_2 _relativelocation_y_2 _move) false false)
      (`SceneComponent.K2_SetRelativeLocation` _pushingcyl4 (`KismetMathLibrary.MakeVector` _relativelocation_x_3 _relativelocation_y_3 _move2) false false)
      (`SceneComponent.K2_SetRelativeLocation` _pushingcyl5 (`KismetMathLibrary.MakeVector` _relativelocation_x_4 _relativelocation_y_4 _move2) false false)
      (`SceneComponent.K2_SetRelativeLocation` _pushingcyl6 (`KismetMathLibrary.MakeVector` _relativelocation_x _relativelocation_y _move2) false false))))

(event `self.Box.OnComponentBeginOverlap`
  (params (OverlappedComponent :type "PrimitiveComponent Object Reference") (OtherActor :type "Actor Object Reference") (OtherComp :type "PrimitiveComponent Object Reference") (OtherBodyIndex :type Integer) (bFromSweep :type Boolean) (SweepResult :type "HitResult Structure (by ref)"))
  (bind _portalplace (`self.PortalPlace`))
  (bind _portalplace2 (`self.PortalPlace2`))
  (bind _portalplace3 (`self.PortalPlace3`))
  (bind _portalplace4 (`self.PortalPlace4`))
  (bind (_relativelocation_x _relativelocation_y) (`KismetMathLibrary.BreakVector` (`SceneComponent.RelativeLocation` _portalplace)))
  (bind (_relativelocation_x_2 _relativelocation_y_2) (`KismetMathLibrary.BreakVector` (`SceneComponent.RelativeLocation` _portalplace2)))
  (bind (_relativelocation_x_3 _relativelocation_y_3) (`KismetMathLibrary.BreakVector` (`SceneComponent.RelativeLocation` _portalplace3)))
  (bind (_relativelocation_x_4 _relativelocation_y_4) (`KismetMathLibrary.BreakVector` (`SceneComponent.RelativeLocation` _portalplace4)))
  (bind (_direction _move) (`Timeline|Timeline`)
    (:`Update`
      ;[1 1 1] 1차 트리거
      (`SceneComponent.K2_SetRelativeLocation` _portalplace (`KismetMathLibrary.MakeVector` _relativelocation_x _relativelocation_y _move) false false)
      (`SceneComponent.K2_SetRelativeLocation` _portalplace2 (`KismetMathLibrary.MakeVector` _relativelocation_x_2 _relativelocation_y_2 _move) false false)
      (`SceneComponent.K2_SetRelativeLocation` _portalplace3 (`KismetMathLibrary.MakeVector` _relativelocation_x_3 _relativelocation_y_3 _move) false false)
      (`SceneComponent.K2_SetRelativeLocation` _portalplace4 (`KismetMathLibrary.MakeVector` _relativelocation_x_4 _relativelocation_y_4 _move) false false))))

(fn `UserConstructionScript`)